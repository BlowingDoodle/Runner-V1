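; BP_Wall is an interactable wall actor that raises itself vertically when triggered.
; BeginPlay caches its starting location and computes a target 350 units above it.
; The Interact event plays the MoveUp timeline, whose Movement track lerps the actor between the two points with a swept move.
; The timeline only plays forward, with no logic to lower the wall again.
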(event EventBeginPlay
  (|CallParentFunction)
  (bind _output_get (Variables|Default|SetStartLoc (Transformation|GetActorLocation)))
  (Variables|Default|SetTargetLoc (+ _output_get "0.000000,0.000000,350.000000")))

(event Collision|EventActorBeginOverlap
  (params (OtherActor :type Actor%20Object%20Reference))
  (|CallParentFunction OtherActor) ; This node is disabled and will not be called.\nDrag off pins to build functionality.
)

(event EventTick
  (params (DeltaSeconds :type Float%20%28single-precision%29))
  (|CallParentFunction DeltaSeconds) ; This node is disabled and will not be called.\nDrag off pins to build functionality.
)

(event EventInteract
  (bind _movement (Timeline|MoveUp Play)
    (:Update
      (Transformation|SetActorLocation (Math|Vector|Lerp(Vector) (Variables|Default|GetStartLoc) (Variables|Default|GetTargetLoc) _movement) true false))))

(fn ConstructionScript
  (|CallParentFunction))