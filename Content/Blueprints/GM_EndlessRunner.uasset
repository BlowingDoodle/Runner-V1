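; Game mode for an endless runner that builds a chain of track tiles.
; On BeginPlay it takes the first BP_BaseTile found in the level, hands it a reference to itself and reads its SpawnPoint location.
; SpawnTiles then appends a given number of tiles, starting with four, each placed at the previous tile's SpawnPoint and given the same game mode reference.
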(event EventBeginPlay
  (bind _outactors (Actor|GetAllActorsOfClass "/Game/Blueprints/Runner/BP_BaseTile.BP_BaseTile_C"))
  (bind _output_get (Variables|Default|SetBaseTileRef (Utilities|Array|Get(acopy) _outactors)))
  (Variables|/Game/Blueprints/Runner/BP_BaseTile.BP_BaseTile_C|SetGameModeRef _output_get self)
  (Variables|Default|SetNextSpawnPoint (Transformation|GetWorldLocation (Variables|/Game/Blueprints/Runner/BP_BaseTile.BP_BaseTile_C|GetSpawn_Point _output_get)))
  (CallFunction|SpawnTiles 4))

(fn ConstructionScript)

(fn SpawnTiles
  (params (Amount :type Integer))
  (for _index (range 0 (- Amount 1))
    (bind _returnvalue (Game|SpawnActorfromClass "/Game/Blueprints/Runner/BP_BaseTile.BP_BaseTile_C" (Math|Transform|MakeTransform (Variables|Default|GetNextSpawnPoint) "0, 0, 0" "1.000000,1.000000,1.000000") "Undefined" "MultiplyWithRoot" 0 0))
    (Variables|/Game/Blueprints/Runner/BP_BaseTile.BP_BaseTile_C|SetGameModeRef _returnvalue self)
    (Variables|Default|SetNextSpawnPoint (Transformation|GetWorldLocation (Variables|/Game/Blueprints/Runner/BP_BaseTile.BP_BaseTile_C|GetSpawn_Point _returnvalue)))))